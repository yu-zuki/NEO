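; BP_Lancer is an enemy character that reacts to damage and dies when its health runs out.
; AnyDamage subtracts from HP, then calls a hit reaction while HP is zero or above, or a death event once it drops below.
; Each event checks that its montage is not already playing, then plays it with an upward launch and debug print.
; Death also destroys the actor after a short delay.
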(event Custom|Dearh
  (if (not (Animation|Montage|MontageIsPlaying (Components|SkeletalMesh|GetAnimInstance (Variables|Character|GetMesh)) "/Game/0102/Enemy/air/death.death"))
    (Animation|PlayAnimMontage "/Game/0102/Enemy/air/death.death" 1.0 "None")
    (Utilities|FlowControl|Sequence
      (:then_0
        (Development|PrintString "guwaaa")
        (Character|LaunchCharacter "0.000000,0.000000,500.000000" false false))
      (:then_1
        (Utilities|FlowControl|Delay 2.0)
        (Actor|DestroyActor)))))

(event Custom|Damage
  (if (not (Animation|Montage|MontageIsPlaying (Components|SkeletalMesh|GetAnimInstance (Variables|Character|GetMesh)) "/Game/0102/Enemy/Lancer/Damage_Reaction.Damage_Reaction"))
    (Character|LaunchCharacter "0.000000,0.000000,200.000000" false false)
    (Animation|PlayAnimMontage "/Game/0102/Enemy/Lancer/Damage_Reaction.Damage_Reaction" 1.0 "None")
    (Development|PrintString "Ite")))

(event EventBeginPlay)

(event Collision|EventActorBeginOverlap
  (params (OtherActor :type Actor%20Object%20Reference)))

(event EventTick
  (params (DeltaSeconds :type Float%20%28single-precision%29)))

(event Game|Damage|EventAnyDamage
  (params (Damage :type Float%20%28single-precision%29) (DamageType :type Damage%20Type%20Object%20Reference) (InstigatedBy :type Controller%20Object%20Reference) (DamageCauser :type Actor%20Object%20Reference))
  (bind _output_get (Variables|Default|SetHP (- (Variables|Default|GetHP) Damage)))
  (if (>= _output_get 0.0)
    (CallFunction|Damage)
    (else
      (CallFunction|Dearh))))

(fn ConstructionScript)