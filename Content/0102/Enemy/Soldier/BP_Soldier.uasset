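; BP_Soldier is an enemy soldier character that takes damage, reacts and dies.
; AnyDamage reduces HP, playing a hit-reaction montage while health remains or a death montage at zero, each guarded against replaying mid-montage.
; Death disables movement, then launches the character sideways after the montage completes and destroys it following a delay.
; Capsule overlap passes through a DoOnce to apply fixed damage when the player character is involved.
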(event OnComponentBeginOverlap(Capsule)
  (params (OverlappedComponent :type Primitive%20Component%20Object%20Reference) (OtherActor :type Actor%20Object%20Reference) (OtherComp :type Primitive%20Component%20Object%20Reference) (OtherBodyIndex :type Integer) (bFromSweep :type Boolean) (SweepResult :type Hit%20Result%20Structure%20%28by%20ref%29))
  (Utilities|FlowControl|DoOnce false
    (:Completed
      (if (== 0 (Game|GetPlayerCharacter 0))
        (Game|Damage|ApplyDamage 0 1e+01 0 0)))))

(event Custom|Dearh
  (if (not (Animation|Montage|MontageIsPlaying (Components|SkeletalMesh|GetAnimInstance (Variables|Character|GetMesh)) "/Game/0102/Enemy/air/death.death"))
    (Pawn|Components|CharacterMovement|DisableMovement (Variables|Character|GetCharacterMovement))
    (Animation|Montage|PlayMontage (Variables|Character|GetMesh) "/Game/0102/Enemy/air/death.death"
      (:OnCompleted
        (Character|LaunchCharacter "0.000000,1000.000000,0.000000" false false)
        (Utilities|FlowControl|Delay 4.0)
        (Actor|DestroyActor)))))

(event Custom|Damage
  (if (not (Animation|Montage|MontageIsPlaying (Components|SkeletalMesh|GetAnimInstance (Variables|Character|GetMesh)) "/Game/0102/Enemy/Lancer/Damage_Reaction.Damage_Reaction"))
    (Animation|Montage|PlayMontage (Variables|Character|GetMesh) "/Game/0102/Enemy/Lancer/Damage_Reaction.Damage_Reaction")))

(event EventBeginPlay)

(event Collision|EventActorBeginOverlap
  (params (OtherActor :type Actor%20Object%20Reference)))

(event EventTick
  (params (DeltaSeconds :type Float%20%28single-precision%29)))

(event Game|Damage|EventAnyDamage
  (params (Damage :type Float%20%28single-precision%29) (DamageType :type Damage%20Type%20Object%20Reference) (InstigatedBy :type Controller%20Object%20Reference) (DamageCauser :type Actor%20Object%20Reference))
  (bind _output_get (Variables|Default|SetHP (- (Variables|Default|GetHP) Damage)))
  (if (> _output_get 0.0)
    (CallFunction|Damage)
    (else
      (CallFunction|Dearh))))

(fn ConstructionScript)