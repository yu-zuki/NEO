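; BP_Blade is a moving blade hazard that applies fixed damage to overlapping actors without the Enemy tag.
; Tick pushes it along a local offset scaled by Mult, a simple movement with no sweep.
; NewFunction, Right and Left define a back-and-forth patrol along world Y with rotation flips, but the event graph never calls them.
; SetDir stores an attack direction in MoveDir, which no graph here reads.
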(event OnComponentBeginOverlap(Box)
  (params (OverlappedComponent :type Primitive%20Component%20Object%20Reference) (OtherActor :type Actor%20Object%20Reference) (OtherComp :type Primitive%20Component%20Object%20Reference) (OtherBodyIndex :type Integer) (bFromSweep :type Boolean) (SweepResult :type Hit%20Result%20Structure%20%28by%20ref%29))
  (if (not (Actor|ActorHasTag OtherActor "Enemy"))
    (Game|Damage|ApplyDamage OtherActor 3e+01 0 0)))

(event EventTick
  (params (DeltaSeconds :type Float%20%28single-precision%29))
  (Transformation|AddActorLocalOffset (* (Variables|Default|Getspeed) (Variables|Default|GetMult)) false false) ; 簡易的に動かすノード
)

(fn ConstructionScript)

(fn NewFunction
  (bind _returnvalue (Transformation|GetActorLocation))
  (Variables|Default|Setr (Math|Vector|MakeVector (.x _returnvalue) (+ (Variables|Default|GetDir) (.y _returnvalue)) (.z _returnvalue)))
  (Variables|Default|Setl (Math|Vector|MakeVector (.x _returnvalue) (- (.y _returnvalue) (Variables|Default|GetDir)) (.z _returnvalue))))

(fn Right
  (Transformation|SetActorRotation "0.000000,180.000000,0.000000")
  (Transformation|SetActorLocation (+ (* (Math|Vector|Normalize (- (Variables|Default|Getr) (Transformation|GetActorLocation))) (Variables|Default|Getspeed)) (Transformation|GetActorLocation)) false false)
  (if (>= (.y (Transformation|GetActorLocation)) (.y (Variables|Default|Getr)))
    (Variables|Default|SetMove%20To%20Right false)))

(fn Left
  (Transformation|SetActorRotation "0, 0, 0")
  (Transformation|SetActorLocation (+ (* (Math|Vector|Normalize (- (Variables|Default|Getl) (Transformation|GetActorLocation))) (Variables|Default|Getspeed)) (Transformation|GetActorLocation)) false false)
  (if (<= (.y (Transformation|GetActorLocation)) (.y (Variables|Default|Getl)))
    (Variables|Default|SetMove%20To%20Right true)))

(fn SetDir
  (params (AttackDir :type Vector))
  (Variables|Default|SetMoveDir AttackDir))