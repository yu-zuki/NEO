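; BP_Gun is a gun actor that shows pickup cues while it lies at rest, neither held nor falling.
; Each Tick, a pair of DoOnce nodes that reset each other toggles the Niagara effect only when that resting state changes.
; Tick also shows the Widget component's UI only when the gun is at rest and within hold distance, and hides it otherwise.
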(event EventBeginPlay)

(event Collision|EventActorBeginOverlap
  (params (OtherActor :type Actor%20Object%20Reference)))

(event EventTick
  (params (DeltaSeconds :type Float%20%28single-precision%29))
  (Utilities|FlowControl|Sequence
    (:then_0
      (if (and (not (Class|WeaponBase|GetIsHeld)) (not (Class|WeaponBase|GetIsFalling)))
        (Utilities|FlowControl|DoOnce false :!label _label
          (:Completed
            (Rendering|SetVisibility (Variables|Default|GetNiagara) true false)
            (goto _label_2 Reset)))
        (else
          (Utilities|FlowControl|DoOnce false :!label _label_2
            (:Completed
              (Rendering|SetVisibility (Variables|Default|GetNiagara) false false)
              (goto _label Reset))))))
    (:then_1
      (if (and (Class|WeaponBase|GetIsHoldDistance) (and (not (Class|WeaponBase|GetIsHeld)) (not (Class|WeaponBase|GetIsFalling))))
        (Widget|SetVisibility (UserInterface|GetWidget (Variables|Default|GetWidget)) "Visible")
        (else
          (Widget|SetVisibility (UserInterface|GetWidget (Variables|Default|GetWidget)) "Hidden"))))))

(fn ConstructionScript)