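; Player character Blueprint with a fixed-angle camera and a switchable fire, water or leaf aura.
; BeginPlay sets walk speed, and Tick pins the camera boom's height, depth and rotation so it follows the character only along Y.
; IA_Pose cycles the Niagara asset on AttributeAura, while Tick also prints the Bjump state as debug output.
; A paused widget menu for picking the aura by stick angle is left disconnected.
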(event Input|EnhancedActionEvents|EnhancedInputActionIA_Pose
  (params (ActionValue :type Boolean) (ElapsedSeconds :type Float%20%28double-precision%29) (TriggeredSeconds :type Float%20%28double-precision%29) (InputAction :type Input%20Action%20Object%20Reference :default "/Game/0122/Player/Input/Actions/IA_Pose.IA_Pose"))
  (:Started
    (bind _result (Math|Integer|IncrementInt (Variables|Default|GetInt))
      (:%20%20
        (bind _output_get (Variables|Default|SetInt _result))
        (if (== _output_get 3)
          (Variables|Default|SetInt 0))
        (if (== (Variables|Default|GetInt) 0)
          (Variables|Default|SetIn%20Asset "/Game/0122/Player/Effect/Aura/FireAuraNiagaraSystem.FireAuraNiagaraSystem")
          (elif (== (Variables|Default|GetInt) 1)
            (Variables|Default|SetIn%20Asset "/Game/0122/Player/Effect/Aura/WaterAuraNiagaraSystem.WaterAuraNiagaraSystem")
            (else
              (Variables|Default|SetIn%20Asset "/Game/0122/Player/Effect/Aura/LeafAuraNiagaraSystem.LeafAuraNiagaraSystem"))))
        (Class|NiagaraComponent|SetAsset (Variables|Default|GetAttribute%20Aura) (Variables|Default|GetIn%20Asset) true)))))

(event Input|EnhancedActionEvents|EnhancedInputAction
  (params (ActionValue :type Vector%202D%20Structure) (ElapsedSeconds :type Float%20%28double-precision%29) (TriggeredSeconds :type Float%20%28double-precision%29) (InputAction :type Input%20Action%20Object%20Reference :default "IA_Look")))

(event EventBeginPlay
  (Variables|Default|SetAs%20Aircombo%20Eziki 0)
  (Variables|/Script/Engine.CharacterMovementComponent|SetMaxWalkSpeed (Variables|Character|GetCharacterMovement) 1e+03))

(event Collision|EventActorBeginOverlap
  (params (OtherActor :type Actor%20Object%20Reference)))

(event EventTick
  (params (DeltaSeconds :type Float%20%28single-precision%29))
  (bind _returnvalue (Class|MyProjectCharacter|Bjump))
  (bind _cameraboom (Variables|Default|GetCameraBoom))
  (if _returnvalue
    (Development|PrintString (Utilities|String|ToString(Boolean) _returnvalue)))
  (Transformation|SetWorldLocation _cameraboom (Math|Vector|MakeVector 1e+03 (.Y (Math|Vector|BreakVector (Transformation|GetActorLocation))) 2e+02) false false)
  (Transformation|SetWorldRotation _cameraboom "-15.000000,0.000000,0.000000" false false))

(fn ConstructionScript)