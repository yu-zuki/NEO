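; Experimental sword player character with a side-on follow camera, dash, switchable fire/water/leaf aura and an air combo.
; Two attack inputs pick a montage, and a MultiGate steps through three sections, launching upward on the second, with SaveAttack and ResetCombo controlling chaining.
; Sphere-overlap hits deal damage that doubles per check and bounce the airborne player; an ultimate multiplies damage tenfold.
; The attribute also picks the sword trail; stick/widget-based switching is disconnected.
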(event Custom|Attack
  (bind _combo (Variables|Default|GetCombo))
  (Input|DisableInput 0)
  (Utilities|FlowControl|MultiGate false false -1
    (:Out%200
      (Animation|PlayAnimMontage _combo 1.0 "First"))
    (:Out%201
      (Character|LaunchCharacter "0.000000,0.000000,800.000000" false false)
      (Animation|PlayAnimMontage _combo 1.0 "Second"))
    (:Out%202
      (Animation|PlayAnimMontage _combo 1.0 "Third"))))

(event Custom|Reset
  (bind _combo (Variables|Default|GetCombo))
  (Utilities|FlowControl|MultiGate false false -1) ; enters at Reset
)

(event Custom|Save%20Attack
  (Input|EnableInput 0)
  (Variables|Default|SetbInput true))

(event Custom|ResetCombo
  (Variables|Default|SetbInput false)
  (Variables|Default|SetIs%20Attacking false)
  (Variables|Default|SetCanCombo false)
  (Variables|Default|Setdamage 2.0)
  (CallFunction|Reset)
  (Input|EnableInput 0))

(event Custom|StartEffect
  (params (Start :type Boolean))
  (CallFunction|SwordEffect Start))

(event Custom|Collision
  (params (CollisionSize :type Float%20%28double-precision%29))
  (CallFunction|SetCollision CollisionSize))

(event Custom|FinEffect
  (params (Fin :type Boolean))
  (CallFunction|SwordEffect Fin))

(event Input|EnhancedActionEvents|EnhancedInputActionIA_WeakPunch
  (params (ActionValue :type Boolean) (ElapsedSeconds :type Float%20%28double-precision%29) (TriggeredSeconds :type Float%20%28double-precision%29) (InputAction :type Input%20Action%20Object%20Reference :default "/Game/Player/Input/Actions/IA_WeakPunch.IA_WeakPunch"))
  (:Started
    (Variables|Default|SetCombo "/Game/Player/Animation/Montage/Combo/sword/SwordCombo2.SwordCombo2")
    (if (Variables|Default|GetIs%20Attacking)
      (if (Variables|Default|GetbInput)
        (Variables|Default|SetCanCombo true)
        (CallFunction|Attack))
      (else
        (Variables|Default|SetIs%20Attacking true)
        (CallFunction|Attack)))))

(event Input|EnhancedActionEvents|EnhancedInputActionIA_Pose
  (params (ActionValue :type Boolean) (ElapsedSeconds :type Float%20%28double-precision%29) (TriggeredSeconds :type Float%20%28double-precision%29) (InputAction :type Input%20Action%20Object%20Reference :default "/Game/Player/Input/Actions/IA_Pose.IA_Pose"))
  (:Started
    (bind _result (Math|Integer|IncrementInt (Variables|Default|GetInt))
      (:%20%20
        (bind _output_get (Variables|Default|SetInt _result))
        (if (== _output_get 3)
          (Variables|Default|SetInt 0))
        (if (== (Variables|Default|GetInt) 0)
          (Variables|Default|SetIn%20Asset "/Game/Player/Effect/Aura/FireAuraNiagaraSystem.FireAuraNiagaraSystem")
          (elif (== (Variables|Default|GetInt) 1)
            (Variables|Default|SetIn%20Asset "/Game/Player/Effect/Aura/WaterAuraNiagaraSystem.WaterAuraNiagaraSystem")
            (else
              (Variables|Default|SetIn%20Asset "/Game/Player/Effect/Aura/LeafAuraNiagaraSystem.LeafAuraNiagaraSystem"))))
        (Class|NiagaraComponent|SetAsset (Variables|Default|GetattributeAura) (Variables|Default|GetIn%20Asset) true)))))

(event Input|EnhancedActionEvents|EnhancedInputActionIA_Look
  (params (ActionValue :type Vector%202D%20Structure) (ElapsedSeconds :type Float%20%28double-precision%29) (TriggeredSeconds :type Float%20%28double-precision%29) (InputAction :type Input%20Action%20Object%20Reference :default "/Game/Player/Input/Actions/IA_Look.IA_Look")))

(event Input|EnhancedActionEvents|EnhancedInputActionIA_HardPunch
  (params (ActionValue :type Boolean) (ElapsedSeconds :type Float%20%28double-precision%29) (TriggeredSeconds :type Float%20%28double-precision%29) (InputAction :type Input%20Action%20Object%20Reference :default "/Game/Player/Input/Actions/IA_HardPunch.IA_HardPunch"))
  (:Started
    (Variables|Default|SetCombo "/Game/Player/Animation/Montage/Combo/sword/SwordCombo.SwordCombo")
    (if (Variables|Default|GetIs%20Attacking)
      (if (Variables|Default|GetbInput)
        (Variables|Default|SetCanCombo true)
        (CallFunction|Attack))
      (else
        (Variables|Default|SetIs%20Attacking true)
        (CallFunction|Attack)))))

(event Input|EnhancedActionEvents|EnhancedInputActionIA_Dash
  (params (ActionValue :type Boolean) (ElapsedSeconds :type Float%20%28double-precision%29) (TriggeredSeconds :type Float%20%28double-precision%29) (InputAction :type Input%20Action%20Object%20Reference :default "/Game/Player/Input/Actions/IA_Dash.IA_Dash"))
  (bind _charactermovement (Variables|Character|GetCharacterMovement))
  (bind _velocity (Variables|/Script/Engine.MovementComponent|GetVelocity _charactermovement))
  (bind (_x _y) (Math|Vector|BreakVector _velocity))
  (:Triggered
    (if (or (> _x 0.0) (> _y 0.0))
      (Variables|/Script/Engine.CharacterMovementComponent|SetMaxWalkSpeed (Variables|Character|GetCharacterMovement) 1.5e+03)))
  (:Completed
    (Variables|/Script/Engine.CharacterMovementComponent|SetMaxWalkSpeed (Variables|Character|GetCharacterMovement) 1e+03)))

(event Input|EnhancedActionEvents|EnhancedInputActionIA_ULT
  (params (ActionValue :type Boolean) (ElapsedSeconds :type Float%20%28double-precision%29) (TriggeredSeconds :type Float%20%28double-precision%29) (InputAction :type Input%20Action%20Object%20Reference :default "/Game/Player/Input/Actions/IA_ULT.IA_ULT"))
  (:Started
    (Input|DisableInput 0)
    (Animation|Montage|PlayMontage (Variables|Character|GetMesh) "/Game/Player/Animation/Montage/hissatu.hissatu"
      (:then
        (Variables|Default|Setdamage (* (Variables|Default|Getdamage) 1e+01)))
      (:OnCompleted
        (Input|EnableInput 0)))))

(event EventBeginPlay
  (Variables|Default|SetAs%20Aircombo%20Eziki 0)
  (Variables|/Script/Engine.CharacterMovementComponent|SetMaxWalkSpeed (Variables|Character|GetCharacterMovement) 1e+03))

(event Collision|EventActorBeginOverlap
  (params (OtherActor :type Actor%20Object%20Reference)))

(event EventTick
  (params (DeltaSeconds :type Float%20%28single-precision%29))
  (bind _cameraboom (Variables|Default|GetCameraBoom))
  (Transformation|SetWorldLocation _cameraboom (Math|Vector|MakeVector 1e+03 (.Y (Math|Vector|BreakVector (Transformation|GetActorLocation))) 2e+02) false false)
  (Transformation|SetWorldRotation _cameraboom "-15.000000,0.000000,0.000000" false false))

(fn ConstructionScript)

(fn SetCollision
  (params (CollisionSize :type Float%20%28double-precision%29))
  (bind (_outactors _returnvalue) (Collision|SphereOverlapActors (+ (Transformation|GetActorLocation) "0.000000,50.000000,0.000000") CollisionSize (Utilities|Array|MakeArray "ObjectTypeQuery3") 0 (Utilities|Array|MakeArray self)))
  (if _returnvalue
    (for _array_element _outactors
      (Game|Damage|ApplyDamage _array_element (Variables|Default|Getdamage) 0 0)
      (CameraShakes|StartCameraShake (Game|GetPlayerCameraManager 0) "/Game/Player/Blueprints/sword/camerashake.camerashake_C" 1.0 "CameraLocal" "0, 0, 0")
      (if (AI|Components|NavMovement|IsFalling (Variables|Character|GetCharacterMovement))
        (Character|LaunchCharacter "0.000000,0.000000,300.000000" false false))))
  (Variables|Default|Setdamage (* (Variables|Default|Getdamage) 2.0)))

(fn KauntEnemy)

(fn SwordEffect
  (params (IsTrailSpown :type Boolean))
  (bind _swordtrailfire (Variables|Default|GetSwordTrailFire))
  (if IsTrailSpown
    (switch int (Variables|Default|GetInt)
      (:0
        (Class|NiagaraComponent|SetAsset _swordtrailfire "/Game/Player/Effect/SwordTrailFire.SwordTrailFire" true))
      (:1
        (Class|NiagaraComponent|SetAsset _swordtrailfire "/Game/Player/Effect/SwordTrailIce.SwordTrailIce" true))
      (:2
        (Class|NiagaraComponent|SetAsset _swordtrailfire "/Game/Player/Effect/SwordTrailWind.SwordTrailWind" true)))
    (else
      (Class|NiagaraComponent|SetAsset _swordtrailfire 0 true))))